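; StarHUD is a HUD that draws a forced-release progress meter above the StarPawn's current grab location.
; BeginPlay creates a dynamic instance of the meter material and caches the owning StarPawn.
; While progress is above zero, DrawHUD projects a point raised above the grab location to screen space, then draws a glow backdrop and a smaller centered meter whose Amount parameter follows the progress.
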(event `self.ReceiveBeginPlay`
  (bind _returnvalue (`KismetMaterialLibrary.CreateDynamicMaterialInstance` "/Game/Materials/HUDMeterMat.HUDMeterMat"))
  (set `self.MeterMat` _returnvalue)
  (bind _asstar_pawn (cast `/Game/Blueprints/StarPawn` (`self.GetOwningPawn`)))
  (set `self.Pawn` _asstar_pawn))

(event `self.ReceiveDrawHUD`
  (params (SizeX :type Integer) (SizeY :type Integer))
  (bind _metermat (`self.MeterMat`))
  (bind _pawn (`self.Pawn`))
  (bind _progress (`/Game/Blueprints/StarPawn.GetForcedReleaseProgress` _pawn))
  (if (> _progress 0.0)
    (bind _location (`/Game/Blueprints/StarPawn.GetCurrentGrabLocation` _pawn))
    (bind _returnvalue (`self.Project` (+ _location (0.0 0.0 240.0))))
    (bind (_returnvalue_x _returnvalue_y) (`KismetMathLibrary.BreakVector` (- _returnvalue 30.0)))
    (`self.DrawMaterialSimple` "/Game/Materials/HUDMeterGlowMat.HUDMeterGlowMat" _returnvalue_x _returnvalue_y 60.0 60.0)
    (`MaterialInstanceDynamic.SetScalarParameterValue` _metermat "Amount" _progress)
    (bind (_returnvalue_x_2 _returnvalue_y_2) (`KismetMathLibrary.BreakVector` (- _returnvalue 20.0)))
    (`self.DrawMaterial` _metermat _returnvalue_x_2 _returnvalue_y_2 40.0 40.0 0.0 0.0 1.0 1.0 1.0 false 0.0 (0.5 0.5))))

(fn `UserConstructionScript`)