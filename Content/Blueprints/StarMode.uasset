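; StarMode watches the player's StarPawn and lifts it back up whenever it falls below a height threshold.
; BeginPlay caches the pawn, and Tick checks the world height of its ArmAnchor.
; Past the threshold, every arm mesh, the anchor and the constraint actors teleport up by the same vertical offset, keeping the physics assembly's layout.
; Linear velocities on the arms and anchor are zeroed, while angular velocity is left untouched.
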(event `self.ReceiveBeginPlay`
  (bind _asstar_pawn (cast `/Game/Blueprints/StarPawn` (`Controller.K2_GetPawn` (`GameplayStatics.GetPlayerController` 0))))
  (set `self.Pawn` _asstar_pawn))

(event `self.ReceiveTick`
  (params (DeltaSeconds :type "Float (single-precision)"))
  (bind _returnvalue (`KismetMathLibrary.MakeVector` 0.0 0.0 3400.0))
  (bind _pawn (`self.Pawn`))
  (bind _armanchor (`/Game/Blueprints/StarPawn.ArmAnchor` _pawn))
  (bind (_returnvalue_x _returnvalue_y _returnvalue_z) (`KismetMathLibrary.BreakVector` (`SceneComponent.K2_GetComponentLocation` _armanchor)))
  (if (< _returnvalue_z -1200.0)
    (for _array_element (`/Game/Blueprints/StarPawn.Arms` _pawn)
      (bind _armmesh (`/Game/Blueprints/ArmBP.ArmMesh` _array_element))
      (`SceneComponent.K2_AddWorldOffset` _armmesh _returnvalue false true)
      (`PrimitiveComponent.SetAllPhysicsLinearVelocity` _armmesh (0.0 0.0 0.0) false))
    (`SceneComponent.K2_AddWorldOffset` _armanchor _returnvalue false true)
    (`PrimitiveComponent.SetAllPhysicsLinearVelocity` _armanchor (0.0 0.0 0.0) false)
    (for _array_element_2 (`/Game/Blueprints/StarPawn.ArmConstraints` _pawn)
      (`self.K2_AddActorWorldOffset` _array_element_2 _returnvalue false true))))

(fn `UserConstructionScript`)