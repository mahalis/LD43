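; Player pawn for a five-armed star creature that swings by grabbing objects, losing the grabbing arm on each release and regrowing one from arm pickups.
; Arms are spawned radially as separate actors, joined to the anchor by limited physics constraints.
; While grab is held, the arm nearest a grabbable attempts it; completed grabs detach on release or timeout.
; Tick applies X/Z swing force, scaled by remaining arm count and boosted while attached.
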(event `self.ReceiveBeginPlay`
  (`self.MakeArms` 5))

(event `self.ReceiveTick`
  (params (DeltaSeconds :type "Float (single-precision)"))
  (`self.AttemptGrabIfNeeded`)
  (`self.HandleMovementInput`)
  (`self.DoForcedReleaseIfNeeded`))

(event `InputAction|Grab`
  (params (Key :type "Key Structure"))
  (bind _grabbingarmindex (`self.GrabbingArmIndex`))
  (:`Pressed`
    (set `self.WantsGrab` true))
  (:`Released`
    (set `self.WantsGrab` false)
    (if (`self.IsGrabbing`)
      (if (`self.ArmHasActuallyGrabbed`)
        (`self.DetachArm` (`self.GrabbingArmIndex`))
        (set `self.LastReleaseTime` (`GameplayStatics.GetTimeSeconds`)))
      (elif (!= _grabbingarmindex -1)
        (`/Game/Blueprints/ArmBP.CancelGrab` (`|GetArrayItem` (`self.Arms`) _grabbingarmindex))))))

(event `self.ReceiveActorBeginOverlap`
  (params (OtherActor :type "Actor Object Reference"))
  (bind _asarm_pickup (cast `/Game/Blueprints/ArmPickup` OtherActor))
  (`self.TouchedArmPickup` _asarm_pickup))

(fn `AttemptGrabIfNeeded`
  (locals (BestArmDistance :type "Float (double-precision)" :default 0.0) (BestArmIndex :type Integer :default -1))
  (bind _bestarmindex (`local.BestArmIndex`))
  (if (and (`self.WantsGrab`) (not (`self.IsGrabbing`)) (not (`self.ArmHasActuallyGrabbed`)))
    (for (_array_element _array_index) (`self.Arms`)
      (bind _squareddistance (`/Game/Blueprints/ArmBP.GetBestGrabbableDistance` _array_element))
      (if (and (> _squareddistance 0.0) (or (< _squareddistance (`local.BestArmDistance`)) (== (`local.BestArmIndex`) -1)))
        (set `local.BestArmIndex` _array_index)
        (set `local.BestArmDistance` _squareddistance)))
    (if (!= _bestarmindex -1)
      (`/Game/Blueprints/ArmBP.BeginGrab` (`|GetArrayItem` (`self.Arms`) _bestarmindex))
      (set `self.GrabbingArmIndex` _bestarmindex))))

(fn `DetachArm`
  (params (Index :type Integer))
  (returns (Arm :type "/Game/Blueprints/ArmBP Object Reference"))
  (bind _arms (`self.Arms`))
  (bind _armconstraints (`self.ArmConstraints`))
  (bind _output (`|GetArrayItem` _arms Index))
  (bind _output_2 (`|GetArrayItem` _armconstraints Index))
  (`PhysicsConstraintComponent.BreakConstraint` (`PhysicsConstraintActor.ConstraintComp` _output_2))
  (`self.K2_DestroyActor` _output_2) ; destroy constraint
  (`/Game/Blueprints/ArmBP.NoteDetached` _output)
  (`KismetArrayLibrary.Array_AddUnique` (`self.EmptyPositionIndices`) (`/Game/Blueprints/ArmBP.PositionIndex` _output))
  (set `self.GrabbingArmIndex` -1)
  (`KismetArrayLibrary.Array_Remove` _arms Index)
  (`KismetArrayLibrary.Array_Remove` _armconstraints Index)
  (for (_array_element _array_index) (`self.Arms`)
    (set `/Game/Blueprints/ArmBP.ListIndex` _array_index _array_element))
  (set `self.NextForcedReleaseTime` -1.0)
  (set `self.ArmHasActuallyGrabbed` false)
  (return _output))

(fn `DoForcedReleaseIfNeeded`
  (bind _nextforcedreleasetime (`self.NextForcedReleaseTime`))
  (if (and (`self.IsGrabbing`) (> (`GameplayStatics.GetTimeSeconds`) _nextforcedreleasetime) (> _nextforcedreleasetime 0.0))
    (`self.DetachArm` (`self.GrabbingArmIndex`))))

(fn `GetCurrentGrabLocation`
  (returns (Location :type "Vector Structure"))
  (if (`self.IsGrabbing`)
    (return (`self.K2_GetActorLocation` (`/Game/Blueprints/ArmBP.TargetGrabbable` (`|GetArrayItem` (`self.Arms`) (`self.GrabbingArmIndex`)))))
    (else
      (return (0.0 0.0 0.0)))))

(fn `GetForcedReleaseProgress`
  (returns (Progress :type "Float (double-precision)"))
  (bind _nextforcedreleasetime (`self.NextForcedReleaseTime`))
  (return (`KismetMathLibrary.SelectFloat` (/ (- _nextforcedreleasetime (`GameplayStatics.GetTimeSeconds`)) (`self.ForcedReleaseDelay`)) 0.0 (and (> _nextforcedreleasetime 0.0) (`self.IsGrabbing`)))))

(fn `HandleMovementInput`
  (bind _arms (`self.Arms`))
  (bind _returnvalue (`KismetMathLibrary.MakeVector` (`self.GetInputAxisValue`) 0.0 (`self.GetInputAxisValue`)))
  (`PrimitiveComponent.AddForce` (`self.ArmAnchor`) (* (* (select `bool` (> (`KismetMathLibrary.VSizeSquared` _returnvalue) 1.0) :`false` _returnvalue :`true` (`KismetMathLibrary.Normal` _returnvalue)) (* (`KismetMathLibrary.MultiplyMultiply_FloatFloat` (/ (`KismetMathLibrary.Conv_IntToDouble` (+ (`KismetArrayLibrary.Array_Length` _arms) 1)) 6.0) 2.0) (`KismetMathLibrary.SelectFloat` 60000.0 30000.0 (`self.ArmHasActuallyGrabbed`)))) (1.0 0.0 0.5)) "None" true)
  (for _array_element _arms
    _))

(fn `MakeArms`
  (params (Count :type Integer :default 5))
  (for _index (range 5)
    (`self.MakeOneArm` _index)))

(fn `MakeOneArm`
  (params (PositionIndex :type Integer))
  (returns (Result :type "/Game/Blueprints/ArmBP Object Reference"))
  (bind _returnvalue (* PositionIndex (/ 360.0 5.0)))
  (bind _returnvalue_2 (`KismetMathLibrary.ComposeTransforms` (`KismetMathLibrary.MakeTransform` (* (`KismetMathLibrary.MakeVector` (`KismetMathLibrary.DegCos` _returnvalue) (`KismetMathLibrary.DegSin` _returnvalue)) 50.0) (`KismetMathLibrary.MakeRotator` 0.0 0.0 _returnvalue)) (`SceneComponent.K2_GetComponentToWorld` (`self.ArmAnchor`))))
  (bind _returnvalue_3 (`|SpawnActorFromClass` "/Game/Blueprints/ArmBP.ArmBP_C" _returnvalue_2 "AlwaysSpawn" "OverrideRootScale" null null))
  (bind _returnvalue_4 (`KismetArrayLibrary.Array_Add` (`self.Arms`) _returnvalue_3))
  (set `/Game/Blueprints/ArmBP.ListIndex` _returnvalue_4 _returnvalue_3)
  (bind _output_get (set `/Game/Blueprints/ArmBP.PositionIndex` PositionIndex _returnvalue_3))
  (set `/Game/Blueprints/ArmBP.Pawn` self _returnvalue_3)
  (`KismetArrayLibrary.Array_RemoveItem` (`self.EmptyPositionIndices`) _output_get)
  (bind _returnvalue_5 (`|SpawnActorFromClass` "/Script/Engine.PhysicsConstraintActor" _returnvalue_2 "AlwaysSpawn" "OverrideRootScale" null null))
  (`KismetArrayLibrary.Array_Add` (`self.ArmConstraints`) _returnvalue_5)
  (`self.K2_AttachToActor` _returnvalue_5 self "None" "KeepWorld" "KeepWorld" "KeepWorld" true)
  (bind _constraintcomp (`PhysicsConstraintActor.ConstraintComp` _returnvalue_5))
  (`PhysicsConstraintComponent.SetDisableCollision` _constraintcomp true)
  (`PhysicsConstraintComponent.SetAngularSwing2Limit` _constraintcomp "ACM_Limited" 5.0)
  (`PhysicsConstraintComponent.SetAngularSwing1Limit` _constraintcomp "ACM_Limited" 30.0)
  (`PhysicsConstraintComponent.SetConstrainedComponents` _constraintcomp (`/Game/Blueprints/ArmBP.ArmMesh` _returnvalue_3) "Joint_1" (`self.ArmAnchor`) "None")
  (return _returnvalue_3))

(fn `NoteFinishedGrab`
  (set `self.NextForcedReleaseTime` (+ (`GameplayStatics.GetTimeSeconds`) (`self.ForcedReleaseDelay`)))
  (set `self.ArmHasActuallyGrabbed` true))

(fn `PinArm`
  (params (Index :type Integer) (Component :type "StaticMeshComponent Object Reference"))
  (returns (Constraint :type "PhysicsConstraintActor Object Reference"))
  (bind _arms (`self.Arms`))
  (bind _armmesh (`/Game/Blueprints/ArmBP.ArmMesh` (`|GetArrayItem` _arms Index)))
  (if (< Index (`KismetArrayLibrary.Array_Length` _arms))
    (bind _returnvalue (`|SpawnActorFromClass` "/Script/Engine.PhysicsConstraintActor" (`KismetMathLibrary.MakeTransform` (`SceneComponent.GetSocketLocation` _armmesh "Joint_4")) "AlwaysSpawn" "OverrideRootScale" null null))
    (bind _constraintcomp (`PhysicsConstraintActor.ConstraintComp` _returnvalue))
    (`PhysicsConstraintComponent.SetDisableCollision` _constraintcomp true)
    (`PhysicsConstraintComponent.SetConstrainedComponents` _constraintcomp _armmesh "Joint_3" Component "None")
    (set `self.GrabbingArmIndex` Index)
    (set `self.NextForcedReleaseTime` (+ (`GameplayStatics.GetTimeSeconds`) (`self.ForcedReleaseDelay`)))
    (return _returnvalue)))

(fn `RegenerateArm`
  (bind _emptypositionindices (`self.EmptyPositionIndices`))
  (bind _returnvalue (`KismetArrayLibrary.Array_Length` _emptypositionindices))
  (if (> _returnvalue 0)
    (`self.MakeOneArm` (`|GetArrayItem` _emptypositionindices (`KismetMathLibrary.RandomIntegerInRange` 0 (- _returnvalue 1))))))

(fn `Reset`
  (for _array_element (`self.Arms`)
    (`self.K2_DestroyActor` _array_element))
  (for _array_element_2 (`self.ArmConstraints`)
    (`self.K2_DestroyActor` _array_element_2))
  (`KismetArrayLibrary.Array_Clear` (`self.Arms`))
  (`KismetArrayLibrary.Array_Clear` (`self.ArmConstraints`))
  (`KismetArrayLibrary.Array_Clear` (`self.EmptyPositionIndices`))
  (set `self.GrabbingArmIndex` -1)
  (set `self.NextForcedReleaseTime` -1.0))

(fn `TouchedArmPickup`
  (params (Pickup :type "/Game/Blueprints/ArmPickup Object Reference"))
  (if (> (`KismetArrayLibrary.Array_Length` (`self.EmptyPositionIndices`)) 0)
    (`self.RegenerateArm`)
    (`/Game/Blueprints/ArmPickup.Disable` Pickup)))

(fn `UserConstructionScript`)