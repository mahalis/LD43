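; WorldChunk is a level chunk actor that scatters Grabbable actors around itself and has a roof whose collision can be briefly switched off.
; Setup tries twelve spawns across an XZ rectangle using an R2 low-discrepancy sequence with randomized start and stride, skipping spots that stay blocked.
; TemporarilyDisableRoofCollision turns off the Roof's collision and restarts a one-second timer that restores it.
; Teardown destroys only the chunk actor itself.
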(fn `MakeR2Coordinate`
  (params (Index :type Integer))
  (returns (Coordinate :type "Vector2D Structure"))
  (return (`KismetMathLibrary.MakeVector2D` (`KismetMathLibrary.Fraction` (+ (* Index 0.754878) 0.5)) (`KismetMathLibrary.Fraction` (+ (* Index 0.56984) 0.5)))))

(fn `ReenableRoofCollision`
  (`PrimitiveComponent.SetCollisionEnabled` (`self.Roof`) "QueryAndPhysics"))

(fn `Setup`
  (locals (R2StartIndex :type Integer))
  (bind _output_get (set `local.R2StartIndex` (`KismetMathLibrary.RandomInteger` 4000)))
  (for _index (range 12)
    (bind _coordinate (`self.MakeR2Coordinate` (+ _output_get (* _index (`KismetMathLibrary.RandomIntegerInRange` 1 5)))))
    (`|SpawnActorFromClass` "/Game/Blueprints/Grabbable.Grabbable_C" (`KismetMathLibrary.MakeTransform` (+ (`self.K2_GetActorLocation`) (`KismetMathLibrary.MakeVector` (`KismetMathLibrary.Lerp` -3500.0 3500.0 (`KismetMathLibrary.BreakVector2D` _coordinate)) 0.0 (`KismetMathLibrary.Lerp` -800.0 1200.0 (`.Y` (`KismetMathLibrary.BreakVector2D` _coordinate))))) (struct :`Roll` 90.0)) "AdjustIfPossibleButDontSpawnIfColliding" "OverrideRootScale" null null)))

(fn `Teardown`
  (`self.K2_DestroyActor`))

(fn `TemporarilyDisableRoofCollision`
  (`PrimitiveComponent.SetCollisionEnabled` (`self.Roof`) "NoCollision")
  (`KismetSystemLibrary.K2_ClearTimer` null "ReenableRoofCollision")
  (`KismetSystemLibrary.K2_SetTimer` self "ReenableRoofCollision" 1.0))

(fn `UserConstructionScript`)