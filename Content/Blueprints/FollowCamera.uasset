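; Follow camera actor that becomes the player's view target and tracks the controlled StarPawn along X.
; On BeginPlay it caches the pawn; each Tick moves its root to the pawn's ArmAnchor X, keeping Z and zeroing Y.
; ResetToOrigin disables spring arm lag and teleports to zero X/Y.
; Tick restores lag when JustReset is true, but ResetToOrigin sets that flag false.
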(event `self.ReceiveBeginPlay`
  (`self.Setup`))

(event `self.ReceiveTick`
  (params (DeltaSeconds :type "Float (single-precision)"))
  (bind _pawn (`self.Pawn`))
  (bind _defaultsceneroot (`self.DefaultSceneRoot`))
  (bind (_returnvalue_x _returnvalue_y _returnvalue_z) (`KismetMathLibrary.BreakVector` (`SceneComponent.K2_GetComponentLocation` _defaultsceneroot)))
  (bind _returnvalue_x_2 (`KismetMathLibrary.BreakVector` (`SceneComponent.K2_GetComponentLocation` (`/Game/Blueprints/StarPawn.ArmAnchor` _pawn))))
  (if (`self.JustReset`)
    (set `self.JustReset` false)
    (set `SpringArmComponent.bEnableCameraLag` true (`self.SpringArm`)))
  (if (`KismetSystemLibrary.IsValid` _pawn)
    (`SceneComponent.K2_SetWorldLocation` _defaultsceneroot (`KismetMathLibrary.MakeVector` _returnvalue_x_2 0.0 _returnvalue_z) false false)))

(fn `ResetToOrigin`
  (bind _defaultsceneroot (`self.DefaultSceneRoot`))
  (bind (_returnvalue_x _returnvalue_y _returnvalue_z) (`KismetMathLibrary.BreakVector` (`SceneComponent.K2_GetComponentLocation` _defaultsceneroot)))
  (set `SpringArmComponent.bEnableCameraLag` false (`self.SpringArm`))
  (`SceneComponent.K2_SetWorldLocation` _defaultsceneroot (`KismetMathLibrary.MakeVector` 0.0 0.0 _returnvalue_z) false true)
  (set `self.JustReset` false))

(fn `Setup`
  (bind _returnvalue (`GameplayStatics.GetPlayerController` 0))
  (bind _asstar_pawn (cast `/Game/Blueprints/StarPawn` (`Controller.K2_GetPawn` _returnvalue)))
  (set `self.Pawn` _asstar_pawn)
  (`PlayerController.SetViewTargetWithBlend` _returnvalue self 0.0 "VTBlend_Linear" 0.0 false))

(fn `UserConstructionScript`)